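; Sprite-based AI enemy that wanders near its spawn point, chases and attacks the player, and can be stunned or killed.
; DetectionSphere overlaps toggle between wander and chase via AIMoveTo, with a delayed re-check on exit and a cooldown on attacks.
; Tick locks actor rotation, derives a sign-based Directionality, and turns the health bar toward the camera.
; Death darkens the sprite through a timeline, then the enemy hides and respawns at its start location.
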(event OnComponentBeginOverlap(DetectionSphere)
  (params (OverlappedComponent :type Primitive%20Component%20Object%20Reference) (OtherActor :type Actor%20Object%20Reference) (OtherComp :type Primitive%20Component%20Object%20Reference) (OtherBodyIndex :type Integer) (bFromSweep :type Boolean) (SweepResult :type Hit%20Result%20Structure%20%28by%20ref%29))
  (if (not (Variables|Default|GetisDead))
    (bind _asbp_character (Utilities|Casting|CastToBP_Character OtherActor))
    (if (Utilities|IsValid _asbp_character)
      (CallFunction|OverlapStart))))

(event OnComponentEndOverlap(DetectionSphere)
  (params (OverlappedComponent :type Primitive%20Component%20Object%20Reference) (OtherActor :type Actor%20Object%20Reference) (OtherComp :type Primitive%20Component%20Object%20Reference) (OtherBodyIndex :type Integer))
  (if (not (Variables|Default|GetisDead))
    (bind _asbp_character (Utilities|Casting|CastToBP_Character OtherActor))
    (if (Utilities|IsValid _asbp_character)
      (CallFunction|OverlapEnd))))

(event Custom|FollowPlayer
  ;[1 1 1] Follow
  (if (not (Variables|Default|GetisDead))
    (Variables|/Script/Engine.CharacterMovementComponent|SetMaxWalkSpeed (Variables|Character|GetCharacterMovement) (Variables|Default|GetMoveSpeed))
    (if (and (Variables|Default|GetisSensing) (not (Variables|Default|GetisStun))) :!label _label
      (AI|AIMoveTo self "0, 0, 0" (Variables|Default|GetPlayer) (Variables|Default|GetAttackRange) false
        (:OnSuccess
          (CallFunction|Attack)
          (goto _label))))))

(event Custom|TakeDamage
  (params (Damage :type Float%20%28double-precision%29))
  ;[1 1 1] Take Damage
  (if (not (Variables|Default|GetisDead))
    (Audio|PlaySound2D "/Game/04-Sound/SFX/Enemy/Enemy_Hit.Enemy_Hit" 1.0 1.0 0.0 0 0)
    (bind _output_get (Variables|Default|SetHealth (- (Variables|Default|GetHealth) Damage)))
    (Progress|SetPercent (Variables|/Game/02-BluePrint/UI/WB_HPBar.WB_HPBar_C|GetProgressBar_EnemyHP (Variables|Default|GetHPWidget)) (/ _output_get (Variables|Default|GetMaxHealth)))
    (if (<= (Variables|Default|GetHealth) 0.0)
      (CallFunction|Die)
      (else
        (Development|PrintString (Utilities|String|Append "$Enemy Attacked / Health: " (Utilities|String|ToString(Float) (Variables|Default|GetHealth))))))))

(event Custom|Die
  ;[1 1 1] Die
  (Variables|Default|SetisStun false)
  (Variables|Default|SetisSensing false)
  (Variables|Default|SetisDead true)
  (bind _time (Timeline|Died PlayFromStart)
    (:Update
      (Sprite|SetSpriteColor (Variables|Default|GetSprite) (Utilities|Struct|MakeLinearColor _time _time _time 1.0)))
    (:Finished
      (CallFunction|Respawn))))

(event Custom|Stun
  (params (duration :type Float%20%28double-precision%29))
  (bind _animationcomponent (Variables|Default|GetAnimationComponent))
  (bind _animinstance (Variables|/Script/PaperZD.PaperZDAnimationComponent|GetAnimInstance _animationcomponent))
  ;[1 1 1] Stunned
  (if (not (Variables|Default|GetisDead))
    (Development|PrintString "$Enemy Stunned")
    (Variables|Default|SetisStun true)
    (Class|PaperZDAnimInstance|JumptoNode _animinstance "StunEvent" "None")
    (Components|Movement|StopMovementImmediately (Variables|Character|GetCharacterMovement))
    (Utilities|FlowControl|Delay duration)
    (Variables|Default|SetisStun false)
    (Class|PaperZDAnimInstance|JumptoNode _animinstance "IdleEvent" "None")
    (if (Collision|IsOverlappingActor (Variables|Default|GetDetectionSphere) (Variables|Default|GetPlayer) :!class /Script/Engine.PrimitiveComponent)
      (Variables|Default|SetisSensing true)
      (CallFunction|FollowPlayer)
      (else
        (Variables|Default|SetisSensing false)
        (CallFunction|WanderAround)))))

(event Custom|Attack
  ;[1 1 1] Attack
  (if (not (Variables|Default|GetisDead))
    (Utilities|FlowControl|DoOnce false :!label _label
      (:Completed
        (Class|PaperZDAnimInstance|JumptoNode (Variables|/Script/PaperZD.PaperZDAnimationComponent|GetAnimInstance (Variables|Default|GetAnimationComponent)) "AttackEvent" "None")
        (Default|TakeDamage (Variables|Default|GetPlayer) (Variables|Default|GetDamage))
        (Utilities|FlowControl|Delay 2.0)
        (goto _label Reset)))))

(event Custom|SetVariables
  (bind _asbp_character (Utilities|Casting|CastToBP_Character (Game|GetPlayerCharacter 0)))
  (Variables|Default|SetPlayer _asbp_character)
  (Variables|Default|SetStartLocation (Transformation|GetActorLocation)))

(event Custom|WanderAround
  (if (not (Variables|Default|GetisDead))
    (Variables|/Script/Engine.CharacterMovementComponent|SetMaxWalkSpeed (Variables|Character|GetCharacterMovement) (Variables|Default|GetIdleSpeed))
    (bind _randomlocation (Class|NavigationSystemV1|GetRandomLocationinNavigableRadius (Variables|Default|GetStartLocation) 4e+02 0 0))
    (AI|AIMoveTo self _randomlocation 0 5.0 false
      (:OnSuccess
        (Utilities|FlowControl|Delay 2.0)
        (if (not (Variables|Default|GetisSensing))
          (CallFunction|WanderAround))))))

(event Custom|Respawn
  (Rendering|SetVisibility (Variables|Default|GetCapsuleComponent) false true)
  (Collision|SetCollisionEnabled (Variables|Default|GetDetectionSphere) "NoCollision")
  (Utilities|FlowControl|Delay 6e+01)
  (Sprite|SetSpriteColor (Variables|Default|GetSprite) (Utilities|Struct|MakeLinearColor 1.0 1.0 1.0 1.0))
  (Transformation|SetActorLocation (Variables|Default|GetStartLocation) false false)
  (Rendering|SetVisibility (Variables|Default|GetCapsuleComponent) true true)
  (Collision|SetCollisionEnabled (Variables|Default|GetDetectionSphere) "QueryAndPhysics")
  (Variables|Default|SetHealth (Variables|Default|GetMaxHealth))
  (Progress|SetPercent (Variables|/Game/02-BluePrint/UI/WB_HPBar.WB_HPBar_C|GetProgressBar_EnemyHP (Variables|Default|GetHPWidget)) 1.0)
  (Variables|Default|SetisDead false))

(event Custom|OverlapStart
  (Variables|Default|SetisSensing true)
  (CallFunction|FollowPlayer))

(event Custom|OverlapEnd
  (Utilities|FlowControl|Delay 1.0)
  (if (Collision|IsOverlappingActor (Variables|Default|GetDetectionSphere) (Variables|Default|GetPlayer) :!class /Script/Engine.PrimitiveComponent)
    (Variables|Default|SetisSensing true)
    (CallFunction|FollowPlayer)
    (else
      (Variables|Default|SetisSensing false)
      (Components|Movement|StopMovementImmediately (Variables|Character|GetCharacterMovement))
      (CallFunction|WanderAround))))

(event EventBeginPlay
  (CallFunction|SetVariables)
  (CallFunction|WanderAround)
  (bind _aswb_hpbar (Utilities|Casting|CastToWB_HPBar (UserInterface|GetWidget (Variables|Default|GetWidget))))
  (Variables|Default|SetHPWidget _aswb_hpbar))

(event EventTick
  (params (DeltaSeconds :type Float%20%28single-precision%29))
  (bind _returnvalue (Transformation|GetActorLocation))
  (bind _player (Variables|Default|GetPlayer))
  (bind _widget (Variables|Default|GetWidget))
  (bind _returnvalue_2 (Transformation|GetActorLocation _player))
  (bind _returnvalue_3 (- _returnvalue _returnvalue_2))
  (bind (_x _y) (Math|Vector|BreakVector _returnvalue_3))
  (if (not (Variables|Default|GetisDead))
    (Transformation|SetActorRotation "0.000000,-90.000000,0.000000")
    (if (Variables|Default|GetisSensing)
      (Variables|Default|Setdirectionality (Math|Vector2D|MakeVector2D (Math|Float|Sign(Float) _x) (Math|Float|Sign(Float) _y)))
      (else
        (Variables|Default|Setdirectionality (Math|Vector2D|MakeVector2D (Math|Float|Sign(Float) (.X (Math|Vector|BreakVector (- (Transformation|GetActorLocation) (stale Custom|WanderAround _randomlocation))))) (Math|Float|Sign(Float) (.Y (Math|Vector|BreakVector (- (Transformation|GetActorLocation) (stale Custom|WanderAround _randomlocation)))))))))
    (Transformation|SetWorldRotation _widget (Math|Rotator|FindLookatRotation (Transformation|GetWorldLocation _widget) (Camera|GetCameraLocation (Game|GetPlayerCameraManager 0))) false false)))

(fn ConstructionScript)