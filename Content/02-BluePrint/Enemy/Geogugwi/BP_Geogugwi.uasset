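; BP_Geogugwi is an enemy Blueprint that chases and attacks the player, extending parent setup with its own range and speeds.
; An overlap start, ignored while waiting, enables sensing and triggers an AIMoveTo chase if it is alive and unstunned.
; Reaching the player triggers an attack and a recovery stun, while a timeout started alongside the move briefly stuns it if still moving.
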(event Custom|Stop
  (params (duration :type Float%20%28double-precision%29))
  (if (not (Variables|Default|GetisDead))
    (Variables|Default|SetisWaiting true)
    (CallFunction|Stun duration)
    (Utilities|FlowControl|Delay duration)
    (Variables|Default|SetisWaiting false)))

(event EventBeginPlay)

(event Collision|EventActorBeginOverlap
  (params (OtherActor :type Actor%20Object%20Reference)))

(event EventSetVariables
  (|CallParentFunction)
  (Variables|Default|SetAttackRange 1e+01)
  (Variables|Default|SetMoveSpeed 7e+02)
  (Variables|Default|SetIdleSpeed 5e+02))

(event EventFollowPlayer
  ;[1 1 1] Follow
  (if (not (Variables|Default|GetisDead))
    (Variables|Default|SetisMove true)
    (Variables|/Script/Engine.CharacterMovementComponent|SetMaxWalkSpeed (Variables|Character|GetCharacterMovement) (Variables|Default|GetMoveSpeed))
    (if (and (Variables|Default|GetisSensing) (not (Variables|Default|GetisStun)))
      (AI|AIMoveTo self "0, 0, 0" (Variables|Default|GetPlayer) (Variables|Default|GetAttackRange) false
        (:then
          (Utilities|FlowControl|Delay 3.0)
          (if (Variables|Default|GetisMove)
            (CallFunction|Stop 0.5)))
        (:OnSuccess
          (Variables|Default|SetisMove false)
          (CallFunction|Attack)
          (Utilities|FlowControl|Delay 0.5)
          (CallFunction|Stop 2.0))))))

(event EventOverlapStart
  (if (not (Variables|Default|GetisWaiting))
    (Variables|Default|SetisSensing true)
    (CallFunction|FollowPlayer)))

(event EventOverlapEnd)

(fn ConstructionScript)