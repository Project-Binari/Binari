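; BP_Mongdal is the Mongdal enemy, a child Blueprint that adds a repeating stun to inherited enemy behavior.
; BeginPlay runs the parent logic, then sets the walk speed.
; While IsSensing is true, Tick uses a DoOnce gate with delays before and after calling Stun, resetting it to repeat the cycle.
; FollowPlayer calls an empty StunTimer event before deferring to the parent implementation.
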(event Custom|StunTimer)

(event EventBeginPlay
  (|CallParentFunction)
  (Variables|/Script/Engine.CharacterMovementComponent|SetMaxWalkSpeed (Variables|Character|GetCharacterMovement) 3e+02))

(event Collision|EventActorBeginOverlap
  (params (OtherActor :type Actor%20Object%20Reference)))

(event EventFollowPlayer
  (CallFunction|StunTimer)
  (|CallParentFunction))

(event EventTick
  (params (DeltaSeconds :type Float%20%28single-precision%29))
  (|CallParentFunction 0.0)
  (if (Variables|Default|GetisSensing)
    (Utilities|FlowControl|DoOnce false :!label _label
      (:Completed
        (Utilities|FlowControl|Delay 0.5)
        (CallFunction|Stun 0.5)
        (Utilities|FlowControl|Delay 0.6)
        (goto _label Reset)))))

(fn ConstructionScript)