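; BP_Rang is an enemy that fights the player by looping between randomly chosen Dash and Attack skills after short delays.
; Dash runs to the player's position with stun immunity via IsGod, and sphere contact mid-dash stops it and stuns the player.
; Attack snaps onto a character found by a nearby capsule overlap and damages the player, falling back to Dash if none is found.
; Animation states switch through AnimInstance JumpToNode events.
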(event OnComponentBeginOverlap(Sphere)
  (params (OverlappedComponent :type Primitive%20Component%20Object%20Reference) (OtherActor :type Actor%20Object%20Reference) (OtherComp :type Primitive%20Component%20Object%20Reference) (OtherBodyIndex :type Integer) (bFromSweep :type Boolean) (SweepResult :type Hit%20Result%20Structure%20%28by%20ref%29))
  (bind _asbp_character (Utilities|Casting|CastToBP_Character OtherActor))
  (if (Utilities|IsValid _asbp_character)
    (if (Variables|Default|GetisGod)
      (Components|Movement|StopMovementImmediately (Variables|Character|GetCharacterMovement))
      (Default|Stunned _asbp_character)
      (Variables|Default|SetisGod false)
      (Variables|/Script/Engine.CharacterMovementComponent|SetMaxWalkSpeed (Variables|Character|GetCharacterMovement) (Variables|Default|GetDefaultSpeed))
      (Class|PaperZDAnimInstance|JumptoNode (Variables|/Script/PaperZD.PaperZDAnimationComponent|GetAnimInstance (Variables|Default|GetAnimationComponent)) "IdleEvent" "None")
      (CallFunction|ChooseRandomSkill))))

(event Custom|ChooseRandomSkill
  (Utilities|FlowControl|Delay 2.0)
  (switch int (Math|Random|RandomIntegerinRange 0 1)
    (:0
      (CallFunction|Dash))
    (:1
      (CallFunction|Attack))))

(event Custom|Dash
  (Variables|/Script/Engine.CharacterMovementComponent|SetMaxWalkSpeed (Variables|Character|GetCharacterMovement) (Variables|Default|GetDashSpeed))
  (Class|PaperZDAnimInstance|JumptoNode (Variables|/Script/PaperZD.PaperZDAnimationComponent|GetAnimInstance (Variables|Default|GetAnimationComponent)) "DashEvent" "None")
  (Variables|Default|SetisGod true)
  (AI|AIMoveTo self (Transformation|GetActorLocation (Variables|Default|GetPlayer)) 0 5e+01 false
    (:OnSuccess
      (Variables|Default|SetisGod false)
      (Variables|/Script/Engine.CharacterMovementComponent|SetMaxWalkSpeed (Variables|Character|GetCharacterMovement) (Variables|Default|GetDefaultSpeed))
      (Class|PaperZDAnimInstance|JumptoNode (Variables|/Script/PaperZD.PaperZDAnimationComponent|GetAnimInstance (Variables|Default|GetAnimationComponent)) "IdleEvent" "None")
      (CallFunction|ChooseRandomSkill))))

(event EventBeginPlay
  (CallFunction|SetVariables)
  (CallFunction|ChooseRandomSkill))

(event Collision|EventActorBeginOverlap
  (params (OtherActor :type Actor%20Object%20Reference)))

(event EventSetVariables
  (|CallParentFunction)
  (Variables|Default|SetisSensing true)
  (Variables|Default|SetHealth 1000))

(event EventAttack
  (bind _outactors (Collision|CapsuleOverlapActors (Transformation|GetActorLocation) 3e+02 0.0 (Utilities|Array|MakeArray "ObjectTypeQuery3") "/Game/02-BluePrint/Character/BP_Character.BP_Character_C"))
  (if (Utilities|Array|IsValidIndex _outactors)
    (Transformation|SetActorLocation (Transformation|GetActorLocation (Utilities|Array|Get(acopy) _outactors)) false false)
    (Class|PaperZDAnimInstance|JumptoNode (Variables|/Script/PaperZD.PaperZDAnimationComponent|GetAnimInstance (Variables|Default|GetAnimationComponent)) "AttackEvent" "None")
    (Default|TakeDamage (Variables|Default|GetPlayer) (Variables|Default|GetDamage))
    (Utilities|FlowControl|Delay 1.5)
    (CallFunction|ChooseRandomSkill)
    (else
      (CallFunction|Dash))))

(event EventStun
  (params (duration :type Float%20%28double-precision%29))
  (if (not (Variables|Default|GetisGod))
    (|CallParentFunction duration)))

(fn ConstructionScript)