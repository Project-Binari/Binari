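; BP_FlowerWall is a skill actor that acts as a damage aura around the player character.
; It moves to the player's location every Tick, while its Sphere overlap events add and remove BP_Enemy actors in the Enemys array.
; A DoOnce on Tick, reset after a short Delay, applies fixed periodic damage to every enemy in that array.
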(event OnComponentBeginOverlap(Sphere)
  (params (OverlappedComponent :type Primitive%20Component%20Object%20Reference) (OtherActor :type Actor%20Object%20Reference) (OtherComp :type Primitive%20Component%20Object%20Reference) (OtherBodyIndex :type Integer) (bFromSweep :type Boolean) (SweepResult :type Hit%20Result%20Structure%20%28by%20ref%29))
  (bind _asbp_enemy (Utilities|Casting|CastToBP_Enemy OtherActor))
  (Utilities|IsValid _asbp_enemy
    (:Is%20Valid
      (Utilities|Array|Add (Variables|Default|Getenemys) _asbp_enemy))))

(event OnComponentEndOverlap(Sphere)
  (params (OverlappedComponent :type Primitive%20Component%20Object%20Reference) (OtherActor :type Actor%20Object%20Reference) (OtherComp :type Primitive%20Component%20Object%20Reference) (OtherBodyIndex :type Integer))
  (bind _asbp_enemy (Utilities|Casting|CastToBP_Enemy OtherActor))
  (Utilities|IsValid _asbp_enemy
    (:Is%20Valid
      (Utilities|Array|RemoveItem (Variables|Default|Getenemys) _asbp_enemy))))

(event EventBeginPlay
  (Variables|Default|SetPlayer (Game|GetPlayerCharacter 0)))

(event EventTick
  (params (DeltaSeconds :type Float%20%28single-precision%29))
  (Transformation|SetActorLocation (Transformation|GetActorLocation (Variables|Default|GetPlayer)) false false)
  (Utilities|FlowControl|DoOnce false :!label _label
    (:Completed
      (for _array_element (Variables|Default|Getenemys)
        (Default|TakeDamage _array_element 3e+01))
      (Utilities|FlowControl|Delay 0.5)
      (goto _label Reset))))

(fn ConstructionScript)