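; Enemy-type actor for the RangCharm skill, built on a parent enemy class with fixed stats and destroyed by any hit.
; FollowPlayer loops AI MoveTo on the player, triggering a melee attack on arrival, throttled by DoOnce and a delay.
; BeginPlay only prints a debug string; the parent call, follow start and soul/widget facing logic are disconnected.
; Respawn, stun, wander and overlap events are empty overrides.
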(event EventRespawn)

(event EventTakeDamage
  (params (Damage :type Float%20%28double-precision%29))
  (CallFunction|Die))

(event EventFollowPlayer
  (Variables|/Script/Engine.CharacterMovementComponent|SetMaxWalkSpeed (Variables|Character|GetCharacterMovement) (Variables|Default|GetMoveSpeed))
  (AI|AIMoveTo self "0, 0, 0" (Variables|Default|GetPlayer) 1e+01 false :!label _label
    (:OnSuccess
      (CallFunction|Attack)
      (goto _label))))

(event EventBeginPlay
  (Development|PrintString "Hello"))

(event EventTick
  (params (DeltaSeconds :type Float%20%28single-precision%29)))

(event EventSetVariables
  (|CallParentFunction)
  (bind _output_get (Variables|Default|SetMaxHealth 1e+01))
  (Variables|Default|SetHealth _output_get)
  (Variables|Default|SetMoveSpeed 5e+02)
  (Variables|Default|SetDamage 5.0))

(event EventOverlapStart)

(event EventOverlapEnd)

(event EventWanderAround)

(event EventAttack
  (Utilities|FlowControl|DoOnce false :!label _label
    (:Completed
      (Default|TakeDamage (Variables|Default|GetPlayer) (Variables|Default|GetDamage))
      (Utilities|FlowControl|Delay 1.0)
      (goto _label Reset))))

(event EventStun
  (params (duration :type Float%20%28double-precision%29)))

(event EventDie
  (Actor|DestroyActor))

(fn ConstructionScript)