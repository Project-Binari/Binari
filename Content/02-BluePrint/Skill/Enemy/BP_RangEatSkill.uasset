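; BP_RangEatSkill is an enemy skill actor that acts as an area trap, slowing the player and biting on demand.
; Box overlap events turn SlowDown on when a BP_Character enters, caching it as Player, and off when it leaves.
; The CloseMouse event, with no caller in this Blueprint, deals fixed damage to the cached Player if it still overlaps the box.
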(event OnComponentBeginOverlap(Box)
  (params (OverlappedComponent :type Primitive%20Component%20Object%20Reference) (OtherActor :type Actor%20Object%20Reference) (OtherComp :type Primitive%20Component%20Object%20Reference) (OtherBodyIndex :type Integer) (bFromSweep :type Boolean) (SweepResult :type Hit%20Result%20Structure%20%28by%20ref%29))
  (bind _asbp_character (Utilities|Casting|CastToBP_Character OtherActor))
  (Utilities|IsValid _asbp_character
    (:Is%20Valid
      (bind _output_get (Variables|Default|Setplayer _asbp_character))
      (Default|SlowDown _output_get true))))

(event OnComponentEndOverlap(Box)
  (params (OverlappedComponent :type Primitive%20Component%20Object%20Reference) (OtherActor :type Actor%20Object%20Reference) (OtherComp :type Primitive%20Component%20Object%20Reference) (OtherBodyIndex :type Integer))
  (bind _asbp_character (Utilities|Casting|CastToBP_Character OtherActor))
  (Utilities|IsValid _asbp_character
    (:Is%20Valid
      (Default|SlowDown _asbp_character false))))

(event Custom|CloseMouse
  (bind _player (Variables|Default|GetPlayer))
  (if (Collision|IsOverlappingActor (Variables|Default|GetBox) _player :!class /Script/Engine.PrimitiveComponent)
    (Default|TakeDamage _player 2e+01)))

(event EventBeginPlay)

(event Collision|EventActorBeginOverlap
  (params (OtherActor :type Actor%20Object%20Reference)))

(event EventTick
  (params (DeltaSeconds :type Float%20%28single-precision%29)))

(fn ConstructionScript)