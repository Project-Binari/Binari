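; BP_RangGrudgeSkill is a short-lived enemy skill area that damages the player standing inside it, then destroys itself a few seconds after spawning.
; Sphere begin and end overlap events cache the BP_Character and toggle an overlap flag.
; Tick polls that flag through a DoOnce that resets after a Delay, applying periodic damage while overlap lasts and re-checking immediately otherwise.
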(event OnComponentBeginOverlap(Sphere)
  (params (OverlappedComponent :type Primitive%20Component%20Object%20Reference) (OtherActor :type Actor%20Object%20Reference) (OtherComp :type Primitive%20Component%20Object%20Reference) (OtherBodyIndex :type Integer) (bFromSweep :type Boolean) (SweepResult :type Hit%20Result%20Structure%20%28by%20ref%29))
  (bind _asbp_character (Utilities|Casting|CastToBP_Character OtherActor))
  (Utilities|IsValid _asbp_character
    (:Is%20Valid
      (Variables|Default|Setplayer _asbp_character)
      (Variables|Default|SetisPlayerOverlap true))))

(event OnComponentEndOverlap(Sphere)
  (params (OverlappedComponent :type Primitive%20Component%20Object%20Reference) (OtherActor :type Actor%20Object%20Reference) (OtherComp :type Primitive%20Component%20Object%20Reference) (OtherBodyIndex :type Integer))
  (bind _asbp_character (Utilities|Casting|CastToBP_Character OtherActor))
  (Utilities|IsValid _asbp_character
    (:Is%20Valid
      (Variables|Default|SetisPlayerOverlap false))))

(event EventBeginPlay
  (Utilities|FlowControl|Delay 5.0)
  (Actor|DestroyActor))

(event Collision|EventActorBeginOverlap
  (params (OtherActor :type Actor%20Object%20Reference)))

(event EventTick
  (params (DeltaSeconds :type Float%20%28single-precision%29))
  (Utilities|FlowControl|DoOnce false :!label _label
    (:Completed
      (if (Variables|Default|GetisPlayerOverlap)
        (Default|TakeDamage (Variables|Default|Getplayer) 5.0)
        (Utilities|FlowControl|Delay 1.0)
        (goto _label Reset)
        (else
          (goto _label Reset))))))

(fn ConstructionScript)