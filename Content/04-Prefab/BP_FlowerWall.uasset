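; BP_FlowerWall is an actor that follows the player character by matching its full transform every frame.
; BeginPlay caches player character 0, then Tick copies that character's location, rotation and scale onto the actor without sweep or teleport.
; Tick also prints the boolean result of each transform update as debug output.
; The overlap event and construction script are empty.
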(event EventBeginPlay
  (Variables|Default|SetPlayer (Game|GetPlayerCharacter 0)))

(event Collision|EventActorBeginOverlap
  (params (OtherActor :type Actor%20Object%20Reference)))

(event EventTick
  (params (DeltaSeconds :type Float%20%28single-precision%29))
  (bind _returnvalue (Transformation|SetActorTransform (Transformation|GetActorTransform (Variables|Default|GetPlayer))))
  (Development|PrintString (Utilities|String|ToString(Boolean) _returnvalue)))

(fn ConstructionScript)