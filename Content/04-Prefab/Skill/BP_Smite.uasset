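; BP_Smite is a skill actor that damages enemies caught in its box hit area.
; On BeginPlay it reads the player character's Directionality vector and converts it through atan2 into a yaw, offset by 90 degrees, to orient itself.
; When its Box begins overlapping a BP_Enemy, it calls TakeDamage on that enemy with a fixed amount.
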(event OnComponentBeginOverlap(Box)
  (params (OverlappedComponent :type Primitive%20Component%20Object%20Reference) (OtherActor :type Actor%20Object%20Reference) (OtherComp :type Primitive%20Component%20Object%20Reference) (OtherBodyIndex :type Integer) (bFromSweep :type Boolean) (SweepResult :type Hit%20Result%20Structure%20%28by%20ref%29))
  (bind _asbp_enemy (Utilities|Casting|CastToBP_Enemy OtherActor))
  (if (Utilities|IsValid _asbp_enemy)
    (Default|TakeDamage _asbp_enemy 2e+01)))

(event EventBeginPlay
  (bind _asbp_character (Utilities|Casting|CastToBP_Character (Game|GetPlayerCharacter 0)))
  (if true
    (Transformation|SetActorRotation (Math|Rotator|MakeRotator 0.0 0.0 (- (Math|Float|%(Float) (+ (Class|KismetMathLibrary|DegAtan2 (.X (Math|Vector2D|BreakVector2D (Variables|/Game/P_Charcters/BP_Character.BP_Character_C|Getdirectionality _asbp_character))) (.Y (Math|Vector2D|BreakVector2D (Variables|/Game/P_Charcters/BP_Character.BP_Character_C|Getdirectionality _asbp_character)))) 3.6e+02) 3.6e+02) 9e+01)))))

(fn ConstructionScript)