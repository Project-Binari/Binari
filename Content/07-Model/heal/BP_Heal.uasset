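; BP_Heal is a pickup that restores health and mana to a BP_Character that overlaps its Box.
; On overlap it adds fixed HP and MP to the character, then calls Respawn.
; Respawn hides the root and its children, disables Box collision, waits on a timed delay, then restores both, so the same actor is reused rather than destroyed.
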(event OnComponentBeginOverlap(Box)
  (params (OverlappedComponent :type Primitive%20Component%20Object%20Reference) (OtherActor :type Actor%20Object%20Reference) (OtherComp :type Primitive%20Component%20Object%20Reference) (OtherBodyIndex :type Integer) (bFromSweep :type Boolean) (SweepResult :type Hit%20Result%20Structure%20%28by%20ref%29))
  (bind _asbp_character (Utilities|Casting|CastToBP_Character OtherActor))
  (if (Utilities|IsValid _asbp_character)
    (Default|AddHP _asbp_character 1e+01)
    (Default|AddMP _asbp_character 2e+01)
    (CallFunction|Respawn)))

(event Custom|Respawn
  (Rendering|SetVisibility (Variables|Default|GetDefaultSceneRoot) false true)
  (Collision|SetCollisionEnabled (Variables|Default|GetBox) "NoCollision")
  (Utilities|FlowControl|Delay 3e+01)
  (Rendering|SetVisibility (Variables|Default|GetDefaultSceneRoot) true true)
  (Collision|SetCollisionEnabled (Variables|Default|GetBox) "QueryAndPhysics"))

(event EventBeginPlay)

(event Collision|EventActorBeginOverlap
  (params (OtherActor :type Actor%20Object%20Reference)))

(event EventTick
  (params (DeltaSeconds :type Float%20%28single-precision%29)))

(fn ConstructionScript)