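; Base enemy character that detects the player, chases and attacks them, can be damaged or stunned, and grants Soul on death.
; PawnSensing triggers an AI move toward the player unless stunned, and reaching them plays an attack montage node and applies damage behind a two-second DoOnce cooldown.
; Tick halts movement while nothing is sensed, a stun stops it for two seconds, and death awards Soul to BP_Character before destroying the actor.
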(event OnSeePawn(PawnSensing)
  (params (Pawn :type Pawn%20Object%20Reference))
  (Variables|Default|SetisSensing true)
  (CallFunction|FollowPlayer))

(event Custom|FollowPlayer
  ;[1 1 1] Follow
  (if (and (Variables|Default|GetisSensing) (not (Variables|Default|GetisStun)))
    (AI|AIMoveTo self "0, 0, 0" (Game|GetPlayerCharacter 0) 1e+02 false
      (:OnSuccess
        (CallFunction|Attack)))
    (else
      (Utilities|FlowControl|Delay 3.0)
      (Variables|Default|SetisSensing false))))

(event Custom|TakeDamage
  (params (Damage :type Integer))
  ;[1 1 1] Take Damage
  (bind _output_get (Variables|Default|SetHealth (- (Variables|Default|GetHealth) Damage)))
  (if (<= _output_get 0)
    (CallFunction|Die)
    (else
      (Development|PrintString (Utilities|String|Append "$Enemy Attacked / Health: " (Utilities|String|ToString(Integer) _output_get))))))

(event Custom|Die
  ;[1 1 1] Die
  (Default|AddSoul (Variables|Default|GetPlayer) (Variables|Default|GetSoul))
  (Actor|DestroyActor))

(event Custom|Stun
  ;[1 1 1] Stunned
  (Development|PrintString "$Enemy Stunned")
  (Variables|Default|SetisStun true)
  (Components|Movement|StopMovementImmediately (Variables|Character|GetCharacterMovement))
  (Utilities|FlowControl|Delay 2.0)
  (Variables|Default|SetisStun false))

(event Custom|Attack
  ;[1 1 1] Attack
  (Utilities|FlowControl|DoOnce false :!label _label
    (:Completed
      (Animation|PlayAnimMontage 0 1.0 "None")
      (Default|TakeDamage (Variables|Default|GetPlayer) (Variables|Default|GetDamage))
      (Utilities|FlowControl|Delay 2.0)
      (goto _label Reset))))

(event EventBeginPlay
  (Variables|Default|SetHealth 100)
  (Variables|Default|SetDamage 10)
  (Variables|Default|SetSoul 10)
  (Variables|Default|SetDetectionRange 500)
  (Variables|Default|SetisStun false)
  (Variables|Default|SetisSensing false)
  (bind _asbp_character (Utilities|Casting|CastToBP_Character (Game|GetPlayerCharacter 0)))
  (Variables|Default|SetPlayer _asbp_character))

(event Collision|EventActorBeginOverlap
  (params (OtherActor :type Actor%20Object%20Reference)))

(event EventTick
  (params (DeltaSeconds :type Float%20%28single-precision%29))
  (if (not (Variables|Default|GetisSensing))
    (Components|Movement|StopMovementImmediately (Variables|Character|GetCharacterMovement))))

(fn ConstructionScript)