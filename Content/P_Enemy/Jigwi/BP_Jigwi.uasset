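; Jigwi enemy Blueprint whose sprite grows and rises while IsSensing is true, then shrinks and sinks back when it is false.
; It extends parent SetVariables and Tick logic, initializing the sprite's tracked scale and relative location.
; Each Tick nudges both values by fixed, frame-rate-dependent steps, using minimum and maximum scale checks to stop the scaling and vertical movement together.
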(event Collision|EventActorBeginOverlap
  (params (OtherActor :type Actor%20Object%20Reference)))

(event EventTick
  (params (DeltaSeconds :type Float%20%28single-precision%29))
  (|CallParentFunction 0.0)
  (if (Variables|Default|GetisSensing)
    (if (not (Math|Boolean|ANDBoolean (>= (.X (Math|Vector|BreakVector (Variables|Default|GetCurrScale))) 0.4) (>= (.Y (Math|Vector|BreakVector (Variables|Default|GetCurrScale))) 0.4) (>= (.Z (Math|Vector|BreakVector (Variables|Default|GetCurrScale))) 0.4)))
      (bind _output_get (Variables|Default|SetCurrScale (+ (Variables|Default|GetCurrScale) "0.001000,0.001000,0.001000")))
      (Transformation|SetRelativeScale3D (Variables|Default|GetSprite) _output_get)
      (bind _output_get_2 (Variables|Default|SetCurrLocation (+ (Variables|Default|GetCurrLocation) "0.000000,0.000000,0.250000")))
      (Transformation|SetRelativeLocation (Variables|Default|GetSprite) _output_get_2 false false))
    (elif (not (Math|Boolean|ANDBoolean (<= (.X (Math|Vector|BreakVector (Variables|Default|GetCurrScale))) 0.2) (<= (.Y (Math|Vector|BreakVector (Variables|Default|GetCurrScale))) 0.2) (<= (.Z (Math|Vector|BreakVector (Variables|Default|GetCurrScale))) 0.2)))
      (bind _output_get_3 (Variables|Default|SetCurrScale (- (Variables|Default|GetCurrScale) "0.001000,0.001000,0.001000")))
      (Transformation|SetRelativeScale3D (Variables|Default|GetSprite) _output_get_3)
      (bind _output_get_4 (Variables|Default|SetCurrLocation (- (Variables|Default|GetCurrLocation) "0.000000,0.000000,0.250000")))
      (Transformation|SetRelativeLocation (Variables|Default|GetSprite) _output_get_4 false false))))

(event EventSetVariables
  (|CallParentFunction)
  (Variables|Default|SetCurrLocation "0.000000,0.000000,-20.000000")
  (Variables|Default|SetCurrScale "0.200000,0.200000,0.200000"))

(fn ConstructionScript)