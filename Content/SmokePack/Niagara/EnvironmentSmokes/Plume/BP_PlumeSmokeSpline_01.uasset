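; Blueprint actor that places a Niagara plume smoke effect driven by a spline.
; The construction script assigns the Niagara system to the Smoke component and passes the Spline component in as an object parameter.
; It also pushes the actor's lifetime, sprite scale, spawn radius, spawn rate and color variables into the system.
; The event graph has no runtime logic.
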(event EventBeginPlay)

(event Collision|EventActorBeginOverlap
  (params (OtherActor :type Actor%20Object%20Reference)))

(event EventTick
  (params (DeltaSeconds :type Float%20%28single-precision%29)))

(fn ConstructionScript
  (bind _smoke (Variables|Default|GetSmoke))
  (Class|NiagaraComponent|SetAsset (Variables|Default|GetSmoke) (Variables|Default|GetNiagaraSystem) true)
  (Class|NiagaraComponent|SetVariableObject (Variables|Default|GetSmoke) "SplineObject" (Variables|Default|GetSpline))
  (Effects|Components|ParticleSystem|SetFloatParameter _smoke "MaxLifetime" (Variables|Default|GetMaxLifetime))
  (Effects|Components|ParticleSystem|SetFloatParameter _smoke "MinLifetime" (Variables|Default|GetMinLifetime))
  (Effects|Components|ParticleSystem|SetFloatParameter _smoke "MaxScaleSprite" (Variables|Default|GetMaxScaleSprite))
  (Effects|Components|ParticleSystem|SetFloatParameter _smoke "MinScaleSprite" (Variables|Default|GetMinScaleSprite))
  (Effects|Components|ParticleSystem|SetFloatParameter _smoke "SpawnRadius" (Variables|Default|GetSpawnRadius))
  (Effects|Components|ParticleSystem|SetFloatParameter _smoke "SpawnRate" (Variables|Default|GetSpawnRate))
  (Effects|Components|ParticleSystem|SetColorParameter _smoke "Color" (Variables|Default|GetColor)))