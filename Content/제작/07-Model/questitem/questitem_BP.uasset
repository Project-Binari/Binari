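; Quest item pickup that gives the player character an amulet and reveals a linked bridge.
; On BeginPlay it hides the referenced BridgeObj.
; When BP_Character overlaps the Box, the item hides itself, disables the box's collision and calls GetAmulet on the character.
; If the bridge reference is valid, it also plays a paper-item sound, shows the bridge and calls GetAmulet on TransparentWall.
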(event OnComponentBeginOverlap(Box)
  (params (OverlappedComponent :type Primitive%20Component%20Object%20Reference) (OtherActor :type Actor%20Object%20Reference) (OtherComp :type Primitive%20Component%20Object%20Reference) (OtherBodyIndex :type Integer) (bFromSweep :type Boolean) (SweepResult :type Hit%20Result%20Structure%20%28by%20ref%29))
  (bind _bridgeobj (Variables|Default|GetBridgeObj))
  (bind _asbp_character (Utilities|Casting|CastToBP_Character OtherActor))
  (if (Utilities|IsValid _asbp_character)
    (Rendering|SetVisibility (Variables|Default|GetDefaultSceneRoot) false true)
    (Collision|SetCollisionEnabled (Variables|Default|GetBox) "NoCollision")
    (Default|GetAmulet _asbp_character)
    (if (Utilities|IsValid _bridgeobj)
      (Audio|PlaySound2D "/Game/04-Sound/SFX/Object/SFX_PaperItem.SFX_PaperItem" 1.0 1.0 0.0 0 0)
      (Rendering|SetActorHiddenInGame _bridgeobj false)
      (Default|GetAmulet (Variables|Default|GettransparentWall)))))

(event EventBeginPlay
  (bind _bridgeobj (Variables|Default|GetBridgeObj))
  (if (Utilities|IsValid _bridgeobj)
    (Rendering|SetActorHiddenInGame _bridgeobj true)))

(event Collision|EventActorBeginOverlap
  (params (OtherActor :type Actor%20Object%20Reference)))

(event EventTick
  (params (DeltaSeconds :type Float%20%28single-precision%29)))

(fn ConstructionScript)